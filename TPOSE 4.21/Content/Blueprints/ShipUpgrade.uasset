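; ShipUpgrade is an interactable pickup that calls the Ship function on the player's ThirdPersonCharacter.
; Trigger overlap enables input for that character and disables it on exit, while any overlapping actor toggles the TextRender's visibility.
; Pressing E calls Ship, then destroys the Trigger and another component, leaving the actor itself in place.
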(event `self.Trigger.OnComponentBeginOverlap`
  (params (OverlappedComponent :type "PrimitiveComponent Object Reference") (OtherActor :type "Actor Object Reference") (OtherComp :type "PrimitiveComponent Object Reference") (OtherBodyIndex :type Integer) (bFromSweep :type Boolean) (SweepResult :type "HitResult Structure (by ref)"))
  (`|ExecutionSequence`
    (:`then_0`
      (cast `/Game/ThirdPersonBP/Blueprints/ThirdPersonCharacter` OtherActor)
      (`self.EnableInput` (`GameplayStatics.GetPlayerController` 0)))
    (:`then_1`
      (`SceneComponent.SetVisibility` (`self.TextRender`) true false))))

(event `self.Trigger.OnComponentEndOverlap`
  (params (OverlappedComponent :type "PrimitiveComponent Object Reference") (OtherActor :type "Actor Object Reference") (OtherComp :type "PrimitiveComponent Object Reference") (OtherBodyIndex :type Integer))
  (`|ExecutionSequence`
    (:`then_0`
      (cast `/Game/ThirdPersonBP/Blueprints/ThirdPersonCharacter` OtherActor)
      (`self.DisableInput` (`GameplayStatics.GetPlayerController` 0)))
    (:`then_1`
      (`SceneComponent.SetVisibility` (`self.TextRender`) false false))))

(event `Key|E`
  (params (Key :type "Key Structure"))
  (:`Pressed`
    (`|ExecutionSequence`
      (:`then_0`
        (bind _asthird_person_character (cast `/Game/ThirdPersonBP/Blueprints/ThirdPersonCharacter` (`GameplayStatics.GetPlayerCharacter` 0)))
        (`/Game/ThirdPersonBP/Blueprints/ThirdPersonCharacter.+ Ship` _asthird_person_character))
      (:`then_1`
        (`ActorComponent.K2_DestroyComponent` (`self.?`)))
      (:`then_2`
        (`ActorComponent.K2_DestroyComponent` (`self.Trigger`))))))

(fn `UserConstructionScript`)