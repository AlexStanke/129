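; An NPC that tells the player how many ship upgrades they have when approached.
; Overlapping its trigger shows a text render and plays a one-shot talking animation; leaving hides the text and sets the idle animation.
; Every tick it casts the player character to ThirdPersonCharacter and rebuilds the text from its ShipUpgrades value, even while hidden.
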(event `self.trigger.OnComponentBeginOverlap`
  (params (OverlappedComponent :type "PrimitiveComponent Object Reference") (OtherActor :type "Actor Object Reference") (OtherComp :type "PrimitiveComponent Object Reference") (OtherBodyIndex :type Integer) (bFromSweep :type Boolean) (SweepResult :type "HitResult Structure (by ref)"))
  (`|ExecutionSequence`
    (:`then_0`
      (`SceneComponent.SetVisibility` (`self.TextRender`) true false))
    (:`then_1`
      (`SkeletalMeshComponent.PlayAnimation` (`self.SkeletalMesh`) "/Game/Models/Talking_Anim.Talking_Anim" false))))

(event `self.ReceiveTick`
  (params (DeltaSeconds :type "Float (single-precision)"))
  (bind _asthird_person_character (cast `/Game/ThirdPersonBP/Blueprints/ThirdPersonCharacter` (`GameplayStatics.GetPlayerCharacter` 0)))
  (`TextRenderComponent.K2_SetText` (`self.TextRender`) (`KismetTextLibrary.Conv_StringToText` (`KismetStringLibrary.Concat_StrStr` (`KismetStringLibrary.Concat_StrStr` (`self.You have`) (`KismetTextLibrary.Conv_TextToString` (`KismetTextLibrary.Conv_DoubleToText` (`/Game/ThirdPersonBP/Blueprints/ThirdPersonCharacter.Ship Upgrades` _asthird_person_character) "HalfToEven"))) (`self.Ship Upgrades`)))))

(event `self.trigger.OnComponentEndOverlap`
  (params (OverlappedComponent :type "PrimitiveComponent Object Reference") (OtherActor :type "Actor Object Reference") (OtherComp :type "PrimitiveComponent Object Reference") (OtherBodyIndex :type Integer))
  (`|ExecutionSequence`
    (:`then_0`
      (`SceneComponent.SetVisibility` (`self.TextRender`) false false))
    (:`then_1`
      (`SkeletalMeshComponent.SetAnimation` (`self.SkeletalMesh`) "/Game/Models/Idle_Anim.Idle_Anim"))))

(fn `UserConstructionScript`)